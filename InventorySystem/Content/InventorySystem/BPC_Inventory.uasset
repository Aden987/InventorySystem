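; Inventory component that holds items in an array of slot structs, each storing its index and a reference back to the inventory.
; BeginPlay builds the slots from SlotAmount through an event intended for the server.
; AddItemServer calls AddItem, which places the item in the first empty slot through SetItem, then fires OnSlotChanged.
; Full-inventory handling is a TODO that only prints a message and returns false.
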(event `self.ReceiveBeginPlay`
  (`self.SetUpSlotSERVER` (`self.SlotAmount`)))

(event `SetUpSlotSERVER`
  (params (SlotAmount :type Integer))
  ; Set Up Inventory Slots on Server
  (bind _output_get (set `self.SlotAmount` SlotAmount))
  (for _index (range _output_get)
    (`KismetArrayLibrary.Array_Add` (`self.ItemSlots`) (make `/Game/InventorySystem/Structures/S_InventorySlot` :`SlotIndex` _index :`InventoryRef` self))))

(event `AddItemServer`
  (params (ItemToAdd :type "/Game/InventorySystem/Structures/S_InventorySlot Structure"))
  (`self.AddItem` ItemToAdd))

(fn `AddItem`
  (params (ItemToAdd :type "/Game/InventorySystem/Structures/S_InventorySlot Structure"))
  (returns (Successfully :type Boolean))
  (bind (_result _slot) (`self.FindEmptySlot`))
  (if _result
    (`self.SetItem` _slot (`local.ItemToAdd`))
    (else
      (`KismetSystemLibrary.PrintString` "TODO: Inventory is Full")
      (return false))))

(fn `FindEmptySlot`
  (returns (Result :type Boolean) (Slot :type "/Game/InventorySystem/Structures/S_InventorySlot Structure"))
  (for _array_element (`self.ItemSlots`)
    (if (`/Game/InventorySystem/Library/BFL_Inventory.IsSlotEmpty` _array_element)
      (return true _array_element))))

(fn `SetItem`
  (params (TargetSlot :type "/Game/InventorySystem/Structures/S_InventorySlot Structure") (Item :type "/Game/InventorySystem/Structures/S_InventorySlot Structure"))
  (bind ((`SlotIndex_7_08F9A1384DADBC042E9AFC89092F8E1D` _slotindex)) (break `/Game/InventorySystem/Structures/S_InventorySlot` TargetSlot))
  (`KismetArrayLibrary.Array_Set` (`self.ItemSlots`) _slotindex Item)
  (bind _structout (setmembers `/Game/InventorySystem/Structures/S_InventorySlot` :`StructRef` (`|GetArrayItem` (`self.ItemSlots`) _slotindex) :`SlotIndex` _slotindex :`InventoryRef` self))
  (`self.OnSlotChanged` _structout))